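; Gameplay ability that opens the player's attribute menu and closes it when the ability ends.
; On activation it creates a WBP_AttributeMenu widget for player controller 0, adds it to the viewport at a fixed offset and shows the mouse cursor.
; When the ability ends it removes the widget and hides the cursor again.
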(event `self.K2_ActivateAbility`
  (`self.AddWidget`)
  (set `PlayerController.bShowMouseCursor` true (`GameplayStatics.GetPlayerController` 0)))

(event `self.K2_OnEndAbility`
  (params (bWasCancelled :type Boolean))
  (`Widget.RemoveFromParent` (`self.AttributeMenuWidget`))
  (set `PlayerController.bShowMouseCursor` false (`GameplayStatics.GetPlayerController` 0)))

(fn `AddWidget`
  (bind _returnvalue (`|CreateWidget` "/Game/Blueprints/UI/AttributeMenu/WBP_AttributeMenu.WBP_AttributeMenu_C" (`GameplayStatics.GetPlayerController` 0)))
  (bind _output_get (set `self.AttributeMenuWidget` _returnvalue))
  (`UserWidget.AddToViewport` _output_get 0)
  (`UserWidget.SetPositionInViewport` _output_get (50.0 50.0) true))